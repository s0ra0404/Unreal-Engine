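; Player character with Enhanced Input movement, look, jump and sprint, plus HP and point tracking shown on a UW_PlayerUI widget.
; CharacterHitAction adds points and logs hit actor names, while damage drains HP.
; Zero HP or reaching MaxPoint shows a message, clears GameInstance points and reloads the level.
; Tick also teleports fallen players to a fixed position, and destruction notifies BP_MyGameMode through a death dispatcher.
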(event `self.ReceiveControllerChanged`
  (params (OldController :type "Controller Object Reference") (NewController :type "Controller Object Reference"))
  ; 入力を取得
  (bind `_asプレイヤーコントローラー` (cast `PlayerController` NewController))
  (`EnhancedInputSubsystemInterface.AddMappingContext` (pcsubsystem `EnhancedInputLocalPlayerSubsystem` `_asプレイヤーコントローラー`) "/Game/Project/Input/IMC_MyInput.IMC_MyInput" 0 (struct)))

(event `EnhancedInput|/Game/Project/Input/Actions/IA_MyMove`
  (params (ActionValue :type "Vector2D Structure") (ElapsedSeconds :type "Float (double-precision)") (TriggeredSeconds :type "Float (double-precision)") (InputAction :type "InputAction Object Reference" :default "/Game/Project/Input/Actions/IA_MyMove.IA_MyMove"))
  (bind (_returnvalue_roll _returnvalue_pitch _returnvalue_yaw) (`KismetMathLibrary.BreakRotator` (`self.GetControlRotation`)))
  (bind (_returnvalue_roll_2 _returnvalue_pitch_2 _returnvalue_yaw_2) (`KismetMathLibrary.BreakRotator` (`self.GetControlRotation`)))
  ; 移動
  (:`Triggered`
    (`self.AddMovementInput` (`KismetMathLibrary.GetRightVector` (`KismetMathLibrary.MakeRotator` _returnvalue_roll 0.0 _returnvalue_yaw)) ActionValue_X)
    (`self.AddMovementInput` (`KismetMathLibrary.GetForwardVector` (`KismetMathLibrary.MakeRotator` _returnvalue_roll_2 0.0 _returnvalue_yaw_2)) ActionValue_Y)))

(event `EnhancedInput|/Game/Project/Input/Actions/IA_MyJump`
  (params (ActionValue :type Boolean) (ElapsedSeconds :type "Float (double-precision)") (TriggeredSeconds :type "Float (double-precision)") (InputAction :type "InputAction Object Reference" :default "/Game/Project/Input/Actions/IA_MyJump.IA_MyJump"))
  ; ジャンプ
  (:`Started`
    (`self.Jump`))
  (:`Completed`
    (`self.StopJumping`)))

(event `EnhancedInput|/Game/Project/Input/Actions/IA_MyLook`
  (params (ActionValue :type "Vector2D Structure") (ElapsedSeconds :type "Float (double-precision)") (TriggeredSeconds :type "Float (double-precision)") (InputAction :type "InputAction Object Reference" :default "/Game/Project/Input/Actions/IA_MyLook.IA_MyLook"))
  ; カメラ回転制御
  (:`Triggered`
    (`self.AddControllerYawInput` ActionValue_X)
    (`self.AddControllerPitchInput` ActionValue_Y)))

(event `EnhancedInput|/Game/Project/Input/Actions/IA_MySprint`
  (params (ActionValue :type Boolean) (ElapsedSeconds :type "Float (double-precision)") (TriggeredSeconds :type "Float (double-precision)") (InputAction :type "InputAction Object Reference" :default "/Game/Project/Input/Actions/IA_MySprint.IA_MySprint"))
  ; スプリント
  (:`Started`
    (set `CharacterMovementComponent.MaxWalkSpeed` (+ (`CharacterMovementComponent.MaxWalkSpeed` (`self.CharacterMovement`)) 10000.0) (`self.CharacterMovement`)))
  (:`Completed`
    (set `CharacterMovementComponent.MaxWalkSpeed` (- (`CharacterMovementComponent.MaxWalkSpeed` (`self.CharacterMovement`)) 10000.0) (`self.CharacterMovement`))))

(event `Key|K`
  (params (Key :type "Key Structure"))
  ; 文字列配列に保存されているオブジェクト名をすべて表示
  (:`Pressed`
    (for _array_element (`self.HitActorNames`)
      (`KismetSystemLibrary.PrintString` _array_element))))

(event `/Game/Project/Assets/BluePrints/BPI_MyCharacter.CharacterHitAction`
  (params (HitActorName :type String) (Point :type Integer))
  ; 衝突したオブジェクト名を文字配列に保存
  (`self.AddPlayerPoint` Point)
  (`KismetArrayLibrary.Array_Add` (`self.HitActorNames`) HitActorName)
  (bind _result (`/Engine/EditorBlueprintResources/StandardMacros.IncrementInt` (`self.HitCount`))
    (:`  `
      (`KismetSystemLibrary.PrintString` (`KismetStringLibrary.Concat_StrStr` "Hit Count : " (`KismetStringLibrary.Conv_IntToString` _result))))))

(event `self.ReceiveBeginPlay`
  ; UICanvasの表示
  (bind _returnvalue (`|CreateWidget` "/Game/Project/Assets/BluePrints/UW_PlayerUI.UW_PlayerUI_C"))
  (bind _output_get (set `self.PlayerUI` _returnvalue))
  (`UserWidget.AddToViewport` _output_get 0)
  (`self.AddPlayerPoint` (`/Game/Project/Assets/BluePrints/BP_MyGameInstance.PlayerPoint` (`self.MyGameInstance`)))
  (add `self.OnDeadMyCharacter` (delegate `OnDeadMyCharacter_イベント`)))

(event `OnDeadMyCharacter_イベント`
  ; UICanvasの表示
  (bind _asbp_my_game_mode (cast `/Game/Project/Assets/BluePrints/BP_MyGameMode` (`GameplayStatics.GetGameMode`)))
  (`/Game/Project/Assets/BluePrints/BP_MyGameMode.OnMyCharacterDead` _asbp_my_game_mode))

(event `self.ReceiveAnyDamage`
  (params (Damage :type "Float (single-precision)") (DamageType :type "DamageType Object Reference") (InstigatedBy :type "Controller Object Reference") (DamageCauser :type "Actor Object Reference"))
  ; HPをＵＩに表示し、０になったらゲームオーバーテキストを表示します。
  (bind _output_get (set `self.HP` (- (`self.HP`) Damage)))
  (set `ProgressBar.Percent` (/ _output_get (`self.MaxHP`)) (`/Game/Project/Assets/BluePrints/UW_PlayerUI.HPGauge` (`self.PlayerUI`)))
  (if (<= (`ProgressBar.Percent` (`/Game/Project/Assets/BluePrints/UW_PlayerUI.HPGauge` (`self.PlayerUI`))) 0.0)
    (if (not (>= (`ProgressBar.Percent` (`/Game/Project/Assets/BluePrints/UW_PlayerUI.PointGauge` (`self.PlayerUI`))) 1.0))
      (`Widget.SetVisibility` (`/Game/Project/Assets/BluePrints/UW_PlayerUI.RT_GameOverMessage` (`self.PlayerUI`)) "Visible")
      (`self.DisableInput` (`GameplayStatics.GetPlayerController` 0))
      (set `/Game/Project/Assets/BluePrints/BP_MyGameInstance.PlayerPoint` 0 (`self.MyGameInstance`))
      (`KismetSystemLibrary.Delay` 2.0)
      (bind _returnvalue (`GameplayStatics.GetCurrentLevelName` true))
      (`GameplayStatics.OpenLevel` (`KismetStringLibrary.Conv_StringToName` _returnvalue)))))

(event `self.ReceiveDestroyed`
  (`self.OnDeadMyCharacter`))

(event `self.ReceiveTick`
  (params (DeltaSeconds :type "Float (single-precision)"))
  (bind (_returnvalue_x _returnvalue_y _returnvalue_z) (`KismetMathLibrary.BreakVector` (`self.K2_GetActorLocation`)))
  ; プレイヤーの状態検知と状態に応じた処理
  (if (>= (`self.PlayerPoint`) (`self.MaxPoint`))
    (`Widget.SetVisibility` (`/Game/Project/Assets/BluePrints/UW_PlayerUI.RT_CenterMessage` (`self.PlayerUI`)) "Visible")
    (`KismetSystemLibrary.Delay` 2.0)
    (set `/Game/Project/Assets/BluePrints/BP_MyGameInstance.PlayerPoint` 0 (`self.MyGameInstance`))
    (bind _returnvalue (`GameplayStatics.GetCurrentLevelName` true))
    (`GameplayStatics.OpenLevel` (`KismetStringLibrary.Conv_StringToName` _returnvalue))
    (elif (< _returnvalue_z -400.0)
      (`self.K2_SetActorLocationAndRotation` (110.0 80.0 92.0)))))

(fn `AddPlayerPoint`
  (params (Point :type Integer))
  (bind _output_get (set `self.PlayerPoint` (+ Point (`self.PlayerPoint`))))
  (set `ProgressBar.Percent` (/ (`KismetMathLibrary.Conv_IntToDouble` _output_get) 1000.0) (`/Game/Project/Assets/BluePrints/UW_PlayerUI.PointGauge` (`self.PlayerUI`))))

(fn `UserConstructionScript`
  (bind _asbp_my_game_instance (cast `/Game/Project/Assets/BluePrints/BP_MyGameInstance` (`GameplayStatics.GetGameInstance`)))
  (set `self.MyGameInstance` _asbp_my_game_instance))