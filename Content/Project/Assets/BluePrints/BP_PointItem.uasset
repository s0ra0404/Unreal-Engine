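; BP_PointItem is a collectible pickup worth a number of points.
; Its construction script looks up a row in DT_PointItem by name to set the point value and mesh material.
; A timeline started on BeginPlay animates the mesh's yaw and vertical offset.
; On box overlap it passes its display name and points to the other actor through CharacterHitActionMessage, then destroys itself without checking the actor's type.
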(event `self.ReceiveBeginPlay`
  (bind (_direction _rotate _move) (`Timeline|Rotate`)
    (:`Update`
      (if (< (`self.ActorRotateZ`) 360.0)
        (set `self.ActorRotateZ` _rotate)
        (else
          (set `self.ActorRotateZ` 0.0)))
      (`SceneComponent.K2_SetRelativeRotation` (`self.STM_PointItem`) (`KismetMathLibrary.MakeRotator` 0.0 0.0 (`self.ActorRotateZ`)) false false)
      (`SceneComponent.K2_SetRelativeLocation` (`self.STM_PointItem`) (`KismetMathLibrary.MakeVector` 0.0 0.0 _move) false false))))

(event `self.Box.OnComponentBeginOverlap`
  (params (OverlappedComponent :type "PrimitiveComponent Object Reference") (OtherActor :type "Actor Object Reference") (OtherComp :type "PrimitiveComponent Object Reference") (OtherBodyIndex :type Integer) (bFromSweep :type Boolean) (SweepResult :type "HitResult Structure (by ref)"))
  (message `/Game/Project/Assets/BluePrints/BPI_MyCharacter.CharacterHitAction` OtherActor (`KismetSystemLibrary.GetDisplayName` self) (`self.Point`))
  (`self.K2_DestroyActor`))

(fn `UserConstructionScript`
  (locals (NewLocalVar :type Name :default "None"))
  (bind _returnvalue (`|GetDataTableRow` "/Game/Project/Assets/BluePrints/DT_PointItem.DT_PointItem" (`self.PointItemDataName`))
    (:`then`
      (bind (_point _material) (break `/Game/Project/Assets/BluePrints/ST_PointItem` _returnvalue))
      (set `self.Point` _point)
      (`PrimitiveComponent.SetMaterial` (`self.STM_PointItem`) 0 _material))))